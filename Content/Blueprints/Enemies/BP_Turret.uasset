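; BP_Turret is an enemy turret that continuously aims at the first player character; it has no firing logic.
; Each Tick, Bottom interpolates its world yaw toward the player at TurretInterpSpeed.
; Top interpolates elevation from a reversed look-at pitch, clamps it to a limited arc, and applies it as relative roll, implying a mesh whose pitch axis is roll.
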(event EventBeginPlay)

(event Collision|EventActorBeginOverlap
  (params (OtherActor :type Actor%20Object%20Reference)))

(event EventTick
  (params (DeltaSeconds :type Float%20%28single-precision%29))
  (bind _returnvalue (Game|GetPlayerCharacter 0))
  (bind _returnvalue_2 (Utilities|Time|GetWorldDeltaSeconds))
  (bind _turret_interp_speed (Variables|Default|GetTurret%20Interp%20Speed))
  (bind _bottom (Variables|Default|GetBottom))
  (bind _top (Variables|Default|GetTop))
  (bind _returnvalue_3 (Transformation|GetActorLocation _returnvalue))
  (Transformation|SetWorldRotation _bottom (Math|Interpolation|RInterpTo (Math|Rotator|MakeRotator 0.0 0.0 (.yaw (Transformation|GetWorldRotation _bottom))) (Math|Rotator|MakeRotator 0.0 0.0 (.yaw (Math|Rotator|FindLookatRotation (Transformation|GetWorldLocation _bottom) _returnvalue_3))) _returnvalue_2 _turret_interp_speed) false false)
  (Transformation|SetRelativeRotation _top (Math|Rotator|MakeRotator (Math|Float|ClampAngle (.pitch (Math|Interpolation|RInterpTo (Math|Rotator|MakeRotator 0.0 (.roll (Transformation|GetWorldRotation _top)) 0.0) (Math|Rotator|MakeRotator 0.0 (.pitch (Math|Rotator|FindLookatRotation _returnvalue_3 (Transformation|GetWorldLocation _top))) 0.0) _returnvalue_2 _turret_interp_speed)) -5e+01 1e+01) 0.0 0.0) false false))

(fn ConstructionScript)